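; Level tracker for a time attack race that drives lap setup, checkpoint sequence and audio through the player controller.
; On BeginPlay it passes MaxLaps to the controller, numbers and binds the Checkpoints array, activates the first and plays a random music track.
; Each cleared checkpoint calls LapCheck, plays a sound and restarts if the controller reports race completion.
; LapCheck, ActivateCheckpoint, UpdateTimes and RaceCompleteCheck are stubs here.
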(event `self.ReceiveBeginPlay`
  (bind _astime_attack_player_controler (cast `/Game/Blueprints/TimeAttackPlayerControler` (`GameplayStatics.GetPlayerController` 0)))
  (set `self.ControlerRef` _astime_attack_player_controler)
  (`self.Apply Settings`)
  (`self.Start Sequence`))

(event `Apply Settings`
  (bind _controlerref (`self.ControlerRef`))
  ;[1 1 1] Apply Settings
  (set `/Game/Blueprints/TimeAttackPlayerControler.MaxLaps` (`self.MaxLaps`) _controlerref)
  (`self.UpdateTimes`)
  (`/Game/Blueprints/TimeAttackPlayerControler.Start Game Setup` _controlerref))

(event `Start Sequence`
  (bind _checkpoints (`self.Checkpoints`))
  (bind _levelmusic (`self.LevelMusic`))
  ;[1 1 1] Start Sequence
  (for (_array_element _array_index) _checkpoints
    (set `/Game/Blueprints/Checkpoint.NextCheckpointNumber` (+ _array_index 1) _array_element)
    (add `/Game/Blueprints/Checkpoint.CheckpointCleared` _array_element (delegate `Checkpoint Cleared`)))
  (set `self.TotalCheckpoints` (`KismetArrayLibrary.Array_Length` _checkpoints))
  (`self.ActivateCheckpoint` (`|GetArrayItem` _checkpoints))
  (`AudioComponent.Play` (`AmbientSound.AudioComponent` (`|GetArrayItem` _levelmusic (`KismetMathLibrary.RandomIntegerInRange` 0 (- (`KismetArrayLibrary.Array_Length` _levelmusic) 1)))) 0.0))

(event `Checkpoint Cleared`
  (params (NextCheckpoint :type Integer))
  (bind _controlerref (`self.ControlerRef`))
  ;[1 1 1] Checkpoint Cleared
  (`self.LapCheck` NextCheckpoint)
  (`AudioComponent.Play` (`AmbientSound.AudioComponent` (`self.CheckpointSoundFX`)) 0.0)
  (if (`/Game/Blueprints/TimeAttackPlayerControler.isRaceComplete` _controlerref)
    (`/Game/Blueprints/TimeAttackPlayerControler.Restart` _controlerref)))

(fn `ActivateCheckpoint`
  (params (`Next Checkpoint` :type "/Game/Blueprints/Checkpoint Object Reference")))

(fn `LapCheck`
  (params (NextCheckpoint :type Integer)))

(fn `RaceCompleteCheck`
  (returns (isRaceComplete :type Boolean))
  (return false))

(fn `UpdateTimes`)

(fn `UserConstructionScript`)