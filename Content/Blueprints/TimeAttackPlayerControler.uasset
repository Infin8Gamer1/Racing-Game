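; Player controller for a time attack racing mode that tracks laps, lap and race times, and saved best records.
; BeginPlay creates the HUD, caches the vehicle and starts two Timelines that act as race and lap stopwatches.
; Lap updates compare times against bests loaded or defaulted during setup, saving new records to a save slot.
; It also handles vehicle respawn, delayed level restart and an R-key record reset; InitText and UpdateGoals are empty stubs.
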(event `self.ReceiveBeginPlay`
  ;[1 1 1] Event Begin Play
  (bind _returnvalue (`|CreateWidget` "/Game/Blueprints/UI/HUD.HUD_C"))
  (bind _output_get (set `self.HUDRef` _returnvalue))
  (`UserWidget.AddToViewport` _output_get 0)
  (bind _asvehicle_blueprint (cast `/Game/VehicleAdvBP/Blueprints/VehicleBlueprint` (`GameplayStatics.GetPlayerPawn` 0)))
  (set `self.VehicleRef` _asvehicle_blueprint)
  (`self.Start Race Time`)
  (`self.Start Lap Time`))

(event `Start Game Setup`
  ;[1 1 1] Start Game Setup
  (`self.SaveGameCheck`)
  (`self.InitText`))

(event `Restart`
  ;[1 1 1] RestartMap
  (set `self.RaceStart` false)
  (`KismetSystemLibrary.Delay` 6.0)
  (`KismetSystemLibrary.ExecuteConsoleCommand` "RestartLevel" null))

(event `Update Lap`
  ;[1 1 1] Update Lap
  (if (not (`self.isRaceComplete`))
    (bind _output_get (set `self.ActualLap` (+ (`self.ActualLap`) 1)))
    (bind _output_get_2 (set `self.CurrentLapText` (`KismetTextLibrary.Conv_IntToText` _output_get)))
    (`self.LapTimeCheck`)
    (`KismetSystemLibrary.PrintString` (`KismetTextLibrary.Conv_TextToString` _output_get_2))))

(event `Respawn Vehicle`
  ;[1 1 1] Respawn Vehicle
  (bind _returnvalue (`|SpawnActorFromClass` "/Game/VehicleAdvBP/Blueprints/VehicleBlueprint.VehicleBlueprint_C" (`KismetMathLibrary.MakeTransform` (.location (`self.RespawnLocation`)) (.rotation (`self.RespawnLocation`))) "Undefined" "OverrideRootScale" null null))
  (`self.Possess` _returnvalue))

(event `Start Race Time`
  ;[1 1 1] Timers
  (bind (_direction _time) (`Timeline|GameTime` :!label _label)
    (:`Update`
      (bind _output_get (set `self.ActualRaceTime` _time))
      (bind _output_get_2 (set `self.RaceTimeText` (`/Game/Blueprints/TimeConversion.TimeToText` _output_get)))
      (`self.UpdateGoals`)
      (`KismetSystemLibrary.PrintText` _output_get_2 true true (struct :`G` 0.66 :`B` 1.0 :`A` 1.0) 0.1))))

(event `Stop Race Time`
  ;[1 1 1] Timers
  (goto _label :!via `Stop`))

(event `Start Lap Time`
  ;[1 1 1] Timers
  (bind (_direction _time) (`Timeline|LapTime` :!via `PlayFromStart` :!label _label_2)
    (:`Update`
      (set `self.ActualLapTime` _time))))

(event `Stop Lap Time`
  ;[1 1 1] Timers
  (goto _label_2 :!via `Stop`))

(event `Key|R`
  (params (Key :type "Key Structure"))
  ;[1 1 1] Reset Best Lap Times if race not going
  (:`Pressed`
    (if (not (`self.RaceStart`))
      (set `self.BestLapTime` (`self.DefaultBestLapTime`))
      (set `self.BestRaceTime` (`self.DefaultBestRaceTime`))
      (`self.SaveGame`))))

(fn `InitText`)

(fn `LapTimeCheck`
  (`self.Stop Lap Time`)
  (if (<= (`self.ActualLapTime`) (`self.BestLapTime`))
    (bind _output_get (set `self.BestLapTime` (`self.ActualLapTime`)))
    (bind _output_get_2 (set `self.BestLapTimeText` (`/Game/Blueprints/TimeConversion.TimeToText` _output_get)))
    (`self.SaveGame`)
    (`KismetSystemLibrary.PrintText` _output_get_2 true true (struct :`R` 0.040787 :`G` 1.0 :`A` 1.0))
    (set `self.ActualLapTime` 0.0)
    (else
      (set `self.ActualLapTime` 0.0)))
  (if (`self.isRaceComplete`)
    (`self.RaceTimeCheck`)
    (else
      (`self.Start Lap Time`))))

(fn `LoadGame`
  (bind _returnvalue (`GameplayStatics.LoadGameFromSlot` (`self.SaveSlot`)))
  (bind _astime_attack_save_game (cast `/Game/Blueprints/TimeAttackSaveGame` _returnvalue))
  (set `self.BestLapTime` (`/Game/Blueprints/TimeAttackSaveGame.SaveBestLapTime` _astime_attack_save_game))
  (set `self.BestRaceTime` (`/Game/Blueprints/TimeAttackSaveGame.SaveBestRaceTime` _astime_attack_save_game)))

(fn `RaceTimeCheck`
  (if (<= (`self.ActualRaceTime`) (`self.BestRaceTime`))
    (bind _output_get (set `self.BestRaceTime` (`self.ActualRaceTime`)))
    (bind _output_get_2 (set `self.BestRaceTimeText` (`/Game/Blueprints/TimeConversion.TimeToText` _output_get)))
    (`KismetSystemLibrary.PrintText` _output_get_2 true true (struct :`R` 0.032125 :`G` 1.0 :`A` 1.0))
    (`self.SaveGame`)))

(fn `SaveGame`
  (bind _returnvalue (`GameplayStatics.CreateSaveGameObject` "/Game/Blueprints/TimeAttackSaveGame.TimeAttackSaveGame_C"))
  (bind _output_get (set `self.SaveGameRef` _returnvalue))
  (set `/Game/Blueprints/TimeAttackSaveGame.SaveBestLapTime` (`self.BestLapTime`) _output_get)
  (set `/Game/Blueprints/TimeAttackSaveGame.SaveBestRaceTime` (`self.BestRaceTime`) _output_get)
  (`GameplayStatics.SaveGameToSlot` (`self.SaveGameRef`) (`self.SaveSlot`)))

(fn `SaveGameCheck`
  (bind _returnvalue (`GameplayStatics.DoesSaveGameExist` (`self.SaveSlot`)))
  (if _returnvalue
    (`self.LoadGame`)
    (else
      (set `self.BestLapTime` (`self.DefaultBestLapTime`))
      (set `self.BestRaceTime` (`self.DefaultBestRaceTime`))
      (`self.SaveGame`))))

(fn `UpdateGoals`)

(fn `UserConstructionScript`)